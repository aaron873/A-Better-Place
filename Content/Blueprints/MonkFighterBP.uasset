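; Enemy monk fighter AI that attacks the player character assigned by FightManagerBP.
; A delay-driven loop randomly picks a jumping attack or a run-up, kicking when airborne and punching when grounded, then re-aims and repeats.
; Tick drives straight-line movement toward the target's captured position, while punch and kick collision overlaps apply damage.
; Incoming damage updates the manager's health bar widget, and death notifies the manager and disables attack overlaps.
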(event OnComponentBeginOverlap(PunchCollision)
  (params (OverlappedComponent :type Primitive%20Component%20Object%20Reference) (OtherActor :type Actor%20Object%20Reference) (OtherComp :type Primitive%20Component%20Object%20Reference) (OtherBodyIndex :type Integer) (bFromSweep :type Boolean) (SweepResult :type Hit%20Result%20Structure%20%28by%20ref%29))
  ;[1 1 1] Collision
  (bind _asmonk_char_bp (Utilities|Casting|CastToMonkCharBP OtherActor))
  (Game|Damage|ApplyDamage _asmonk_char_bp (Variables|Default|GetPunchDamage) 0 self "/Script/Engine.DamageType")
  (Variables|/Script/Engine.PrimitiveComponent|SetbGenerateOverlapEvents (Variables|Default|GetPunchCollision) false))

(event OnComponentBeginOverlap(KickCollision)
  (params (OverlappedComponent :type Primitive%20Component%20Object%20Reference) (OtherActor :type Actor%20Object%20Reference) (OtherComp :type Primitive%20Component%20Object%20Reference) (OtherBodyIndex :type Integer) (bFromSweep :type Boolean) (SweepResult :type Hit%20Result%20Structure%20%28by%20ref%29))
  ;[1 1 1] Collision
  (bind _asmonk_char_bp (Utilities|Casting|CastToMonkCharBP OtherActor))
  (Game|Damage|ApplyDamage _asmonk_char_bp (Variables|Default|GetPunchDamage) 0 self "/Script/Engine.DamageType")
  (Variables|/Script/Engine.PrimitiveComponent|SetbGenerateOverlapEvents (Variables|Default|GetKickCollision) false))

(event Custom|MainAttackAtPlayer
  ;[1 1 1] Attack Execution
  (bind _returnvalue (Animation|Montage|MontagePlay (Components|SkeletalMesh|GetAnimInstance (Variables|Character|GetMesh)) (CallFunction|KickorPunch) 1.0 "MontageLength" 0.0 true))
  (Utilities|FlowControl|Delay _returnvalue) ; Wait for Punch/Kick
  (CallFunction|CompletedAtk))

(event Custom|ExecuteAttack
  ;[1 1 1] Choosing an attack
  (if (and (not (Variables|Default|GetbIsDead)) (not (Variables|/Game/Blueprints/MonkCharBP.MonkCharBP_C|GetbIsDead (Variables|Default|GetmyTarget))))
    (CallFunction|RotatetoPlayer)
    (switch int (Math|Random|RandomIntegerinRange 0 1) ; Choose atk type
      (:0
        (Variables|Default|SetbBlockPunchAttempt true) ; ATTACK 1: Forward Jump Punch
        (CallFunction|UpdateMovement)
        (Character|Jump)
        (Utilities|FlowControl|Delay 0.2) ; Wait till get in air
        (CallFunction|MainAttackatPlayer))
      (:1
        (CallFunction|UpdateMovement) ; ATTACK 2: Standard Run Punch
      ))))

(event Custom|CompletedAtk
  ;[1 1 1] Attack Execution
  (Variables|Default|SetbIsMoving false)
  (Variables|Default|SetbBlockPunchAttempt false)
  (CallFunction|RotatetoPlayer)
  (Utilities|FlowControl|Delay (Math|Random|RandomFloatinRange 0.75 1.25))
  (CallFunction|ExecuteAttack))

(event EventBeginPlay
  (|VariableInitialization
    (:outExec
      (Utilities|FlowControl|Delay (Math|Random|RandomFloatinRange 0.5 1.0)) ; Wait before beginning to attack (Can be replaced)
      (CallFunction|ExecuteAttack))))

(event EventTick
  (params (DeltaSeconds :type Float%20%28single-precision%29))
  ;[1 1 1] Attack Execution
  (if (and (not (Variables|Default|GetbIsDead)) (Variables|Default|GetbIsMoving))
    (Pawn|Input|AddMovementInput (Variables|Default|GetMovementDirection) 1.0 true)
    (if (CallFunction|ShouldPunch) ; Checks if Fighter is close enough to player and has not alreayd punched
      (CallFunction|MainAttackatPlayer))))

(event Collision|EventHit
  (params (MyComp :type Primitive%20Component%20Object%20Reference) (Other :type Actor%20Object%20Reference) (OtherComp :type Primitive%20Component%20Object%20Reference) (bSelfMoved :type Boolean) (HitLocation :type Vector :default "0, 0, 0") (HitNormal :type Vector :default "0, 0, 0") (NormalImpulse :type Vector :default "0, 0, 0") (Hit :type Hit%20Result%20Structure%20%28by%20ref%29))
  ;[1 1 1] Collision
  (Utilities|Casting|CastToMonkFighterBP Other ; Prevent fighters getting stuck on each other
    (:then
      (CallFunction|CompletedAtk))
    (:CastFailed
      (Utilities|Casting|CastToStaticMeshActor Other ; Keep moving after landing
        (:CastFailed
          (Variables|Default|SetbIsMoving false) ; Stop moving if fighter runs into anything besides another fighter or ground
          (CallFunction|CompletedAtk))))))

(event Game|Damage|EventAnyDamage
  (params (Damage :type Float%20%28single-precision%29) (DamageType :type Damage%20Type%20Object%20Reference) (InstigatedBy :type Controller%20Object%20Reference) (DamageCauser :type Actor%20Object%20Reference))
  ;[1 1 1] On recieve damage
  (if (not (Variables|Default|GetbIsDead))
    (bind _output_get (Variables|Default|SetCurrHealth (- (Variables|Default|GetCurrHealth) Damage)))
    (CallFunction|UpdateHealthBars)
    (if (<= _output_get 0.0) ; If Fighter Died
      (|FighterDied))))

(fn ConstructionScript)

(fn UpdateHealthBars
  (Default|UpdateEnemyHealthBars (Variables|/Game/Blueprints/FightManagerBP.FightManagerBP_C|GetFighterHealthWidget (Variables|Default|GetmyFightManager)) (/ (Variables|Default|GetCurrHealth) (Variables|Default|GetMaxHealth)) (Variables|Default|GetFighterIndex)))

(fn ShouldPunch
  (return (Math|Boolean|ANDBoolean (<= (Math|Float|Absolute(Float) (- (.y (Transformation|GetActorLocation)) (.y (Transformation|GetActorLocation (Variables|Default|GetmyTarget))))) 3e+02) (not (Class|AnimInstance|IsAnyMontagePlaying (Components|SkeletalMesh|GetAnimInstance (Variables|Character|GetMesh)))) (not (Variables|Default|GetbBlockPunchAttempt)))))

(fn RotatetoPlayer
  (Transformation|SetActorRotation (Math|Rotator|MakeRotator 0.0 0.0 (.yaw (Math|Rotator|FindLookatRotation (Transformation|GetActorLocation) (Transformation|GetActorLocation (Variables|Default|GetmyTarget))))) true))

(fn UpdateMovement
  (bind _mytarget (Variables|Default|GetmyTarget))
  (bind _returnvalue (Transformation|GetActorLocation _mytarget))
  (Variables|Default|SetMovementGoal _returnvalue)
  (Variables|Default|SetMovementDirection (Math|Vector|GetForwardVector (Math|Rotator|FindLookatRotation (Transformation|GetActorLocation) _returnvalue)))
  (Variables|Default|SetbIsMoving true))

(fn KickorPunch
  (return (select (AI|Components|NavMovement|IsFalling (Variables|Character|GetCharacterMovement)) "/Game/EinFantasyAssassin/Characters/Animations/MonkKickMontage.MonkKickMontage" "/Game/EinFantasyAssassin/Characters/Animations/MonkPunch_Montage.MonkPunch_Montage")))