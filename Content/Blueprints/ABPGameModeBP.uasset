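; Game mode Blueprint that handles the intro and outro screens and switches the soundtrack.
; On BeginPlay it focuses the viewport, shows the Intro widget, plays menu music and binds to a game-won notification.
; Winning stops the music, clears all widgets and shows the Outro widget.
; PlayMeditationMusic and PlayFightMusic swap sneak or fight cues on the same audio component.
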(event Custom|EventGameWon
  (Audio|Components|Audio|Stop (Variables|Default|GetAudio))
  (Viewport|RemoveAllWidgets)
  (bind _returnvalue (UserInterface|CreateWidget "/Game/HUD/Outro.Outro_C"))
  (UserInterface|Viewport|AddtoViewport _returnvalue 0))

(event EventBeginPlay
  (bind _audio (Variables|Default|GetAudio))
  (Class|WidgetBlueprintLibrary|SetFocustoGameViewport)
  (bind _returnvalue (UserInterface|CreateWidget "/Game/HUD/Intro.Intro_C" (Game|GetPlayerController 0)))
  (UserInterface|Viewport|AddtoViewport _returnvalue 0)
  (Audio|Components|Audio|SetSound _audio "/Game/Sound/soundtrackMenu_Cue.soundtrackMenu_Cue")
  (Audio|Components|Audio|Play _audio 0.0)
  (EventDispatchers|BindEventtoNotifyGameWon (delegate Custom|EventGameWon)))

(fn ConstructionScript)

(fn PlayMeditationMusic
  (bind _audio (Variables|Default|GetAudio))
  (Audio|Components|Audio|Stop _audio)
  (Audio|Components|Audio|SetSound _audio "/Game/Sound/ABPsoundtrackSneak_Cue.ABPsoundtrackSneak_Cue")
  (Audio|Components|Audio|Play _audio 0.0))

(fn PlayFightMusic
  (bind _audio (Variables|Default|GetAudio))
  (Audio|Components|Audio|Stop _audio)
  (Audio|Components|Audio|SetSound _audio "/Game/Sound/ABPsoundtrackFight_Cue.ABPsoundtrackFight_Cue")
  (Audio|Components|Audio|Play _audio 0.0))