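; A meditating monk challenger that moves along a spline path, looping or ping-ponging, and starts a fight when the player monk touches it.
; Overlap halts movement, blends the camera to the monk, opens its eyes, then requests a fight from FightManagerBP and starts fight music.
; A DoOnce blocks duplicate fights until the game mode's fight-ended event resets it.
; LostFight disables collision, line-traces it to the ground and loops a losing animation.
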(event Custom|CallEvent_AllowFight
  (CallFunction|AllowFight)
  (Rendering|Material|SetMaterial (Variables|Default|GetMonkMesh) 2 "/Game/Materials/MI_Monk.MI_Monk"))

(event Custom|AllowFight
  (Utilities|FlowControl|DoOnce false) ; enters at Reset
)

(event Collision|EventActorBeginOverlap
  (params (OtherActor :type Actor%20Object%20Reference))
  (bind _asmonk_char_bp (Utilities|Casting|CastToMonkCharBP OtherActor))
  (Utilities|FlowControl|DoOnce false
    (:Completed
      (Default|SetPreFightLoc _asmonk_char_bp)
      (Variables|Default|SetbShouldMove false)
      (Game|Player|SetViewTargetwithBlend (Game|GetPlayerController 0) self 1.0 "VTBlend_Linear" 1.0 false)
      (Utilities|FlowControl|Delay 1.5) ; Wait for blend time plus little extra
      (Rendering|Material|SetMaterial (Variables|Default|GetMonkMesh) 2 "/Game/Materials/MI_Monk_OpenedEyes.MI_Monk_OpenedEyes")
      (Audio|PlaySound2D "/Game/RPGMagicSFX/Wavs/BasicAttacksImpacts/WAV_Fire_Swoosh_03_Cue.WAV_Fire_Swoosh_03_Cue" 1.0 1.0 0.0 0 0)
      (Utilities|FlowControl|Delay 0.75)
      (Default|EventRequestFight (Variables|Default|GetmyFightManager) OtherActor self (Variables|Default|GetNumMonks))
      (bind _asabpgame_mode_bp (Utilities|Casting|CastToABPGameModeBP (Game|GetGameMode)))
      (Default|PlayFightMusic _asabpgame_mode_bp))))

(event EventTick
  (params (DeltaSeconds :type Float%20%28single-precision%29))
  (bind _returnvalue (Utilities|Time|GetWorldDeltaSeconds))
  (bind _movespeed (Variables|Default|GetmoveSpeed))
  (bind _path (Variables|Default|GetPath))
  (bind _returnvalue_2 (Spline|GetSplineLength _path))
  (bind _returnvalue_3 (* _movespeed _returnvalue))
  (if (Variables|Default|GetbShouldMove)
    (Transformation|SetWorldLocation (Variables|Default|GetMonkMesh) (Spline|GetLocationatDistanceAlongSpline (Variables|Default|GetPath) (Variables|Default|GetcurrDistance) "World") false false)
    (bind _output_get (Variables|Default|SetcurrDistance (Math|Float|Clamp(Float) (+ (Variables|Default|GetcurrDistance) (Math|Float|SelectFloat (* _returnvalue_3 -1.0) _returnvalue_3 (Variables|Default|GetbReverse))) 0.0 _returnvalue_2)))
    (if (>= _output_get _returnvalue_2) ; are we at end?
      (if (Variables|Default|GetbPingPong)
        (Variables|Default|SetbReverse true)
        (else
          (Variables|Default|SetcurrDistance 0.0)))
      (elif (<= _output_get 0.0) ; are we at beginning?
        (Variables|Default|SetbReverse false)))))

(event EventBeginPlay
  (Variables|Default|SetcurrDistance (Variables|Default|GetstartPosition))
  (Variables|Default|SetstartLocation (Transformation|GetActorTransform))
  (bind _outactors (Actor|GetAllActorsOfClass "/Game/Blueprints/FightManagerBP.FightManagerBP_C"))
  (Utilities|IsValid (Utilities|Array|Get(acopy) _outactors)
    (:Is%20Valid
      (Variables|Default|SetmyFightManager (Utilities|Array|Get(acopy) _outactors))
      (bind _asabpgame_mode_bp (Utilities|Casting|CastToABPGameModeBP (Game|GetGameMode)))
      (bind _output_get (Variables|Default|SetMyGame _asabpgame_mode_bp))
      (EventDispatchers|BindEventtoNotifyFightEnded _asabpgame_mode_bp (delegate Custom|CallEvent_AllowFight)) ; Make sure there is no overlapping on monks to cause double the fighters
    )
    (:Is%20Not%20Valid
      (Development|PrintString "No Fight Manager"))))

(fn ConstructionScript
  (Transformation|SetWorldLocation (Variables|Default|GetMonkMesh) (Spline|GetLocationatDistanceAlongSpline (Variables|Default|GetPath) (Variables|Default|GetstartPosition) "World") false false))

(fn LostFight
  (bind _monkmesh (Variables|Default|GetMonkMesh))
  (bind _returnvalue (Transformation|GetWorldLocation _monkmesh))
  (bind (_x _y _z) (Math|Vector|BreakVector _returnvalue))
  (bind _returnvalue_2 (- _x 2e+02))
  (bind _returnvalue_3 (Math|Vector|MakeVector _returnvalue_2 _y _z))
  (Collision|SetCollisionEnabled (Variables|Default|GetSphere) "NoCollision")
  (Variables|Default|SetbShouldMove false)
  (bind _outhit (Collision|LineTraceForObjects _returnvalue_3 (+ _returnvalue_3 (* (Math|Vector|GetUpVector _monkmesh) -1e+04)) (Utilities|Array|MakeArray "ObjectTypeQuery1") false 0 "Persistent"))
  (Transformation|SetWorldLocation (Variables|Default|GetMonkMesh) (Math|Vector|MakeVector (.X (Math|Vector|BreakVector (.Location (Collision|BreakHitResult _outhit)))) (.Y (Math|Vector|BreakVector (.Location (Collision|BreakHitResult _outhit)))) (.Z (Math|Vector|BreakVector (.Location (Collision|BreakHitResult _outhit))))) false false)
  (Components|Animation|PlayAnimation (Variables|Default|GetMonkMesh) "/Game/EinFantasyAssassin/Characters/Animations/monkAnim_lose.monkAnim_lose" true))