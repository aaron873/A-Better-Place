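; Fight manager actor that runs arena fights between the player and monk fighters requested on behalf of a challenger.
; A fight request notifies the player, spawns monks at up to four preset spawn points and shows a health bar HUD.
; Death events count down living combatants to resolve a win or handle player defeat.
; Either result hides the HUD, notifies the game mode and, after a delay, despawns the monks.
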(event Custom|EventRequestFight
  (params (Player :type Actor%20Object%20Reference) (Challenger :type Meditating%20Monk%20BP%20Object%20Reference) (NumCombatants :type Integer))
  (bind _fighterhealthwidget (Variables|Default|GetFighterHealthWidget))
  (if (> NumCombatants 0)
    (bind _asmonk_char_bp (Utilities|Casting|CastToMonkCharBP Player))
    (Default|EventRequestFight _asmonk_char_bp NumCombatants)
    (Variables|Default|SetChallengerCharacter Challenger)
    (bind _output_get (Variables|Default|SetNumCombatants NumCombatants))
    (bind _output_get_2 (Variables|Default|SetLivingCombatants _output_get))
    (CallFunction|SpawnFighters _output_get_2)
    (Default|InitializeHealthBars _fighterhealthwidget _output_get_2)
    (Widget|SetVisibility _fighterhealthwidget "Visible")))

(event Custom|FighterDied
  (bind _result (Math|Integer|DecrementInt (Variables|Default|GetLivingCombatants))
    (:%20%20
      (if (== _result 0) ; If Fight has concluded, Player Winning
        (CallFunction|PostFightScripts)
        (|PlayerWonFight)))))

(event Custom|PlayerDied
  (CallFunction|PostFightScripts)
  (Variables|/Game/Blueprints/MeditatingMonkBP.MeditatingMonkBP_C|SetbShouldMove (Variables|Default|GetChallengerCharacter) true)
  (Utilities|FlowControl|Delay 3.0) ; Wait till player has exited the fight arena before despawning monks
  (bind _outactors (Actor|GetAllActorsOfClass "/Game/Blueprints/MonkFighterBP.MonkFighterBP_C"))
  (for _array_element _outactors
    (Actor|DestroyActor _array_element)))

(event EventBeginPlay
  (Variables|Default|SetFighterSpawnPoints (Utilities|Array|MakeArray (Variables|Default|GetFighterSpawnPoint1) (Variables|Default|GetFighterSpawnPoint2) (Variables|Default|GetFighterSpawnPoint3) (Variables|Default|GetFighterSpawnPoint4)))
  (bind _returnvalue (UserInterface|CreateWidget "/Game/HUD/FightHealthHUD.FightHealthHUD_C"))
  (bind _output_get (Variables|Default|SetFighterHealthWidget _returnvalue))
  (Variables|/Game/HUD/FightHealthHUD.FightHealthHUD_C|SetMyManager _output_get self)
  (UserInterface|Viewport|AddtoViewport _output_get 0)
  (Widget|SetVisibility _output_get "Hidden")
  (bind _asabpgame_mode_bp (Utilities|Casting|CastToABPGameModeBP (Game|GetGameMode)))
  (Variables|Default|SetMyGame _asabpgame_mode_bp))

(fn ConstructionScript)

(fn SpawnFighters
  (params (NumCombatants :type Integer))
  (for _index (range 0 (- NumCombatants 1))
    (Game|SpawnActorfromClass "/Game/Blueprints/MonkFighterBP.MonkFighterBP_C" (Math|Transform|MakeTransform (Transformation|GetWorldLocation (Utilities|Array|Get(acopy) (Variables|Default|GetFighterSpawnPoints) _index)) "0,90.000000, 0" "1,1,1") "Undefined" 0 _index 0)))

(fn PostFightScripts
  (Widget|SetVisibility (Variables|Default|GetFighterHealthWidget) "Hidden")
  (Default|CallNotifyFightEnded (Variables|Default|GetMyGame)))