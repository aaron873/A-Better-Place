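; Player monk character that explores with a smoothed side-view camera and boosted air speed, and teleports into an arena to fight MonkFighterBP enemies.
; Fight requests switch to a tagged fight camera, reset health and set damage by enemy count.
; Attacks play kick montages midair or punches grounded, with collision overlaps applying damage.
; Health updates go through FightManagerBP's widget; victory returns the monk to its pre-fight spot, death to its start.
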(event OnComponentBeginOverlap(PunchCollision)
  (params (OverlappedComponent :type Primitive%20Component%20Object%20Reference) (OtherActor :type Actor%20Object%20Reference) (OtherComp :type Primitive%20Component%20Object%20Reference) (OtherBodyIndex :type Integer) (bFromSweep :type Boolean) (SweepResult :type Hit%20Result%20Structure%20%28by%20ref%29))
  ;[1 1 1] Dealing Damage
  (bind _asmonk_fighter_bp (Utilities|Casting|CastToMonkFighterBP OtherActor))
  (Game|Damage|ApplyDamage _asmonk_fighter_bp (Variables|Default|GetPunchDamage) 0 self "/Script/Engine.DamageType")
  (Variables|/Script/Engine.PrimitiveComponent|SetbGenerateOverlapEvents (Variables|Default|GetPunchCollision) false))

(event OnComponentBeginOverlap(KickCollision)
  (params (OverlappedComponent :type Primitive%20Component%20Object%20Reference) (OtherActor :type Actor%20Object%20Reference) (OtherComp :type Primitive%20Component%20Object%20Reference) (OtherBodyIndex :type Integer) (bFromSweep :type Boolean) (SweepResult :type Hit%20Result%20Structure%20%28by%20ref%29))
  ;[1 1 1] Dealing Damage
  (bind _asmonk_fighter_bp (Utilities|Casting|CastToMonkFighterBP OtherActor))
  (Game|Damage|ApplyDamage _asmonk_fighter_bp (Variables|Default|GetPunchDamage) 0 self "/Script/Engine.DamageType")
  (Variables|/Script/Engine.PrimitiveComponent|SetbGenerateOverlapEvents (Variables|Default|GetKickCollision) false))

(event Custom|EventRequestFight
  (params (NumEnemies :type Integer))
  (bind _myfightloc (Variables|Default|GetmyFightLoc))
  ;[1 1 1] Entering a fight
  (Utilities|FlowControl|Sequence
    (:then_0
      (Variables|Default|SetPreFightLoc (Transformation|GetActorTransform))
      (Transformation|Teleport (.location _myfightloc) (.rotation _myfightloc))
      (Audio|PlaySound2D "/Game/RPGMagicSFX/Wavs/BasicAttacksImpacts/WAV_Fire_Swoosh_03_Cue.WAV_Fire_Swoosh_03_Cue" 1.0 1.0 0.0 0 0))
    (:then_1
      (CallFunction|SetPunchDamage NumEnemies)
      (Variables|Default|SetCurrHealth (Variables|Default|GetMaxHealth))
      (Variables|/Script/Engine.CharacterMovementComponent|SetMaxWalkSpeed (Variables|Character|GetCharacterMovement) (Utilities|Array|Get(acopy) (Variables|Default|GetMaxWalkSpeeds) 1)))
    (:then_2
      (Variables|Default|SetbInFight true)
      (bind _asmonk_anim_bp (Utilities|Casting|CastToMonkAnimBP (Components|SkeletalMesh|GetAnimInstance (Variables|Character|GetMesh))))
      (Variables|/Game/EinFantasyAssassin/Characters/Animations/MonkAnimBP.MonkAnimBP_C|SetbIsInFight _asmonk_anim_bp true)
      (Game|Player|SetViewTargetwithBlend (Game|GetPlayerController 0) (Variables|Default|GetFightCamera) 0.0 "VTBlend_Linear" 0.0 false)
      (Input|EnableInput (Game|GetPlayerController 0))
      (Variables|/Script/Engine.PrimitiveComponent|SetbGenerateOverlapEvents (Variables|Default|GetCapsuleComponent) true))))

(event Custom|WonFight
  ;[1 1 1] Winning a fight
  (Components|Timeline|PlayfromStart (Variables|Default|GetRotateToFront))
  (Game|Player|SetViewTargetwithBlend (Game|GetPlayerController 0) self 1.0 "VTBlend_Linear" 0.0 false)
  (Animation|Montage|MontagePlay (Components|SkeletalMesh|GetAnimInstance (Variables|Character|GetMesh)) "/Game/EinFantasyAssassin/Characters/Animations/MonkVictory_Montage.MonkVictory_Montage" 1.0 "MontageLength" 0.0 true)
  (Utilities|FlowControl|Delay 2.4)
  (CallFunction|ReturntoPagoda (Variables|Default|GetPreFightLoc))
  (bind _asabpgame_mode_bp (Utilities|Casting|CastToABPGameModeBP (Game|GetGameMode)))
  (Default|PlayMeditationMusic _asabpgame_mode_bp))

(event Custom|SetPreFightLoc
  (Variables|Default|SetPreFightLoc (Transformation|GetActorTransform))
  (Components|Movement|StopMovementImmediately (Variables|Character|GetCharacterMovement))
  (Input|DisableInput (Game|GetPlayerController 0))
  (Variables|/Script/Engine.PrimitiveComponent|SetbGenerateOverlapEvents (Variables|Default|GetCapsuleComponent) false))

(event Custom|CameraSway
  ;[1 1 1] Camera Sway
  (bind _returnvalue (Game|SpawnActorfromClass "/Script/Engine.CameraActor" (Transformation|GetWorldTransform (Variables|Default|GetSideViewCamera)) "Undefined" 0 0))
  (Class|CameraComponent|SetConstraintAspectRatio (Variables|/Script/Engine.CameraActor|GetCameraComponent _returnvalue) false)
  (Game|Player|SetViewTargetwithBlend (Game|GetPlayerController 0) _returnvalue 0.0 "VTBlend_Linear" 0.0 false))

(event EventBeginPlay
  ;[1 1 1] Initialization
  (CallFunction|CameraSway)
  (|VariableInitialization))

(event Game|Damage|EventAnyDamage
  (params (Damage :type Float%20%28single-precision%29) (DamageType :type Damage%20Type%20Object%20Reference) (InstigatedBy :type Controller%20Object%20Reference) (DamageCauser :type Actor%20Object%20Reference))
  ;[1 1 1] Recieving Damage
  (bind _output_get (Variables|Default|SetCurrHealth (- (Variables|Default|GetCurrHealth) Damage)))
  (CallFunction|UpdateHealthBar)
  (if (<= _output_get 0.0) ; If Player Died
    (|PlayerDied)))

(event EventOnJumped
  ;[1 1 1] we want lots of air control, because we're monks who are good at defying physics
  (|CallParentFunction)
  (if (not (Variables|Default|GetbInFight))
    (Variables|/Script/Engine.CharacterMovementComponent|SetMaxWalkSpeed (Variables|Character|GetCharacterMovement) 6e+02)))

(event EventOnLanded
  (params (Hit :type Hit%20Result%20Structure%20%28by%20ref%29))
  ;[1 1 1] we want lots of air control, because we're monks who are good at defying physics
  (|CallParentFunction Hit)
  (if (not (Variables|Default|GetbInFight))
    (Variables|/Script/Engine.CharacterMovementComponent|SetMaxWalkSpeed (Variables|Character|GetCharacterMovement) 1e+02)))

(event EventTick
  (params (DeltaSeconds :type Float%20%28single-precision%29))
  ;[1 1 1] Camera Sway
  (Transformation|SetActorTransform (stale Custom|CameraSway _returnvalue) (Class|KismetMathLibrary|TInterpto (Transformation|GetActorTransform (stale Custom|CameraSway _returnvalue)) (Transformation|GetWorldTransform (Variables|Default|GetSideViewCamera)) DeltaSeconds 4.0)))

(event Input|ActionEvents|InputActionAttack
  (params (Key :type Key%20Structure))
  (bind _mesh (Variables|Character|GetMesh))
  (bind _returnvalue (Components|SkeletalMesh|GetAnimInstance _mesh))
  ;[1 1 1] Attack input
  (:Pressed
    (if (and (Variables|Default|GetbInFight) (not (Class|AnimInstance|IsAnyMontagePlaying _returnvalue))) ; If player can punch
      (Animation|Montage|MontagePlay _returnvalue (CallFunction|KickorPunch) 1.0 "MontageLength" 0.0 true))))

(event Input|ActionEvents|InputActionAttackSpecial
  (params (Key :type Key%20Structure))
  ;[1 1 1] Attack input
  (:Pressed
    (if (Variables|Default|GetbInFight)
      _)))

(fn ConstructionScript
  (|CallParentFunction))

(fn UpdateHealthBar
  (Default|UpdatePlayerHealthBar (Variables|/Game/Blueprints/FightManagerBP.FightManagerBP_C|GetFighterHealthWidget (Variables|Default|GetmyFightManager)) (/ (Variables|Default|GetCurrHealth) (Variables|Default|GetMaxHealth))))

(fn SetPunchDamage
  (params (NumEnemies :type Integer))
  (Variables|Default|SetPunchDamage (Utilities|Select :Index NumEnemies :Option%200 0.0 :Option%201 1e+01 :Option%202 17.0 :Option%203 2e+01 :Option%204 34.0)))

(fn ReturntoPagoda
  (params (TeleLocation :type Transform))
  (bind (_outhit _returnvalue) (Collision|LineTraceForObjects (.location TeleLocation) (+ (.location TeleLocation) (* (Transformation|GetActorUpVector) -5e+04)) (Utilities|Array|MakeArray "ObjectTypeQuery1") false 0 "None"))
  (if _returnvalue
    _
    (else
      _))
  (Transformation|Teleport (.location TeleLocation) (.rotation TeleLocation))
  (Input|EnableInput self (Game|GetPlayerController 0))
  (Variables|Default|SetbInFight false)
  (bind _asmonk_anim_bp (Utilities|Casting|CastToMonkAnimBP (Components|SkeletalMesh|GetAnimInstance (Variables|Character|GetMesh))))
  (Variables|/Game/EinFantasyAssassin/Characters/Animations/MonkAnimBP.MonkAnimBP_C|SetbIsInFight _asmonk_anim_bp false)
  (Variables|/Script/Engine.CharacterMovementComponent|SetMaxWalkSpeed (Variables|Character|GetCharacterMovement) (Utilities|Array|Get(acopy) (Variables|Default|GetMaxWalkSpeeds)))
  (Audio|PlaySound2D "/Game/RPGMagicSFX/Wavs/BasicAttacksImpacts/WAV_Fire_Swoosh_03_Cue.WAV_Fire_Swoosh_03_Cue" 1.0 1.0 0.0 0 0)
  (Variables|/Script/Engine.PrimitiveComponent|SetbGenerateOverlapEvents (Variables|Default|GetPunchCollision) false)
  (Variables|/Script/Engine.PrimitiveComponent|SetbGenerateOverlapEvents (Variables|Default|GetKickCollision) false))

(fn KickorPunch
  (return (select (AI|Components|NavMovement|IsFalling (Variables|Character|GetCharacterMovement)) "/Game/EinFantasyAssassin/Characters/Animations/MonkKickMontage.MonkKickMontage" "/Game/EinFantasyAssassin/Characters/Animations/MonkPunch_Montage.MonkPunch_Montage")))